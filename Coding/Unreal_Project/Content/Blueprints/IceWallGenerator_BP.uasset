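; IceWallGenerator_BP spawns a sequence of five IceWall1_BP actors when play begins.
; Five static mesh components act as placement markers, with each wall taking the world transform of the next one.
; SpawnIceWall re-calls itself after a SpawnInterval delay, advancing Index until all five are placed.
; Tick accumulates PlayTime, which only feeds a disconnected debug print.
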(event `self.ReceiveBeginPlay`
  (set `self.IceWallPosArray` (`|MakeArray` (`self.StaticMesh1`) (`self.StaticMesh2`) (`self.StaticMesh3`) (`self.StaticMesh4`) (`self.StaticMesh5`)))
  (`self.SpawnIceWall`))

(event `self.ReceiveTick`
  (params (DeltaSeconds :type "Float (single-precision)"))
  (set `self.PlayTime` (+ (`self.PlayTime`) DeltaSeconds)))

(event `SpawnIceWall`
  (if (< (`self.Index`) 5)
    (`|SpawnActorFromClass` "/Game/Blueprints/IceWall1_BP.IceWall1_BP_C" (`SceneComponent.K2_GetComponentToWorld` (`|GetArrayItem` (`self.IceWallPosArray`) (`self.Index`))) "Undefined" "OverrideRootScale" null null)
    (`KismetSystemLibrary.Delay` (`self.SpawnInterval`))
    (`/Engine/EditorBlueprintResources/StandardMacros.IncrementInt` (`self.Index`)
      (:`  `
        (`self.SpawnIceWall`)))))

(fn `UserConstructionScript`)