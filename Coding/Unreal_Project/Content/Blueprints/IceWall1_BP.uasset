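; Ice wall actor that rises out of a flattened state, stands for a set time, then sinks and removes itself.
; BeginPlay zeroes the mesh's Z scale, and Tick adds GrowingAmount per frame up to full height while IsGrowing is set, so speed depends on frame rate.
; At full height a DoOnce-guarded Delay of SpawnDuration clears IsGrowing, then Tick shrinks the mesh to a low threshold and destroys the actor.
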(event `self.ReceiveBeginPlay`
  (`SceneComponent.SetWorldScale3D` (`self.StaticMesh`) (1.0 1.0 0.0)))

(event `self.ReceiveTick`
  (params (DeltaSeconds :type "Float (single-precision)"))
  (bind (_returnvalue_x _returnvalue_y _returnvalue_z) (`KismetMathLibrary.BreakVector` (`SceneComponent.K2_GetComponentScale` (`self.StaticMesh`))))
  (bind (_returnvalue_x_2 _returnvalue_y_2 _returnvalue_z_2) (`KismetMathLibrary.BreakVector` (`SceneComponent.K2_GetComponentScale` (`self.StaticMesh`))))
  (if (`self.IsGrowing`)
    (if (< _returnvalue_z 1.0)
      (`SceneComponent.SetWorldScale3D` (`self.StaticMesh`) (`KismetMathLibrary.MakeVector` 1.0 1.0 (+ _returnvalue_z (`self.GrowingAmount`))))
      (else
        (`/Engine/EditorBlueprintResources/StandardMacros.DoOnce` false
          (:`Completed`
            (`KismetSystemLibrary.Delay` (`self.SpawnDuration`))
            (set `self.IsGrowing` false)))))
    (elif (> _returnvalue_z_2 0.2)
      (`SceneComponent.SetWorldScale3D` (`self.StaticMesh`) (`KismetMathLibrary.MakeVector` 1.0 1.0 (- _returnvalue_z_2 (`self.GrowingAmount`))))
      (else
        (`/Engine/EditorBlueprintResources/StandardMacros.DoOnce` false
          (:`Completed`
            (`self.K2_DestroyActor`)))))))

(fn `UserConstructionScript`)