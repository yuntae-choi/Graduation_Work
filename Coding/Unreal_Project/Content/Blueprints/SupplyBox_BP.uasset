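; Parachute supply drop that descends at a set fall speed until it lands, and can be farmed by the player character.
; Each tick pins the box to its spawn X/Y and clamps its roll and pitch, so it sways without drifting.
; The first hit breaks the physics constraint, removes the cloth and ropes, and turns off box physics after a short delay.
; Actor overlaps set or clear it as MyCharacter's farmable item.
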(event `self.ReceiveBeginPlay`
  (bind (_returnvalue_x _returnvalue_y) (`KismetMathLibrary.BreakVector` (`SceneComponent.K2_GetComponentLocation` (`self.SupplyBox`))))
  (set `self.SpawnX` _returnvalue_x)
  (set `self.SpawnY` _returnvalue_y))

(event `self.ReceiveTick`
  (params (DeltaSeconds :type "Float (single-precision)"))
  (bind (_returnvalue_x _returnvalue_y _returnvalue_z) (`KismetMathLibrary.BreakVector` (`self.K2_GetActorLocation`)))
  (bind (_returnvalue_x_2 _returnvalue_y_2 _returnvalue_z_2) (`KismetMathLibrary.BreakVector` (`SceneComponent.K2_GetComponentLocation` (`self.SupplyBox`))))
  (bind (_returnvalue_roll _returnvalue_pitch _returnvalue_yaw) (`KismetMathLibrary.BreakRotator` (`SceneComponent.K2_GetComponentRotation` (`self.SupplyBox`))))
  (`SceneComponent.K2_SetWorldLocation` (`self.SupplyBox`) (`KismetMathLibrary.MakeVector` (`self.SpawnX`) (`self.SpawnY`) _returnvalue_z_2) false false)
  (`SceneComponent.K2_SetWorldRotation` (`self.SupplyBox`) (`KismetMathLibrary.MakeRotator` (`KismetMathLibrary.ClampAngle` _returnvalue_roll -20.0 20.0) (`KismetMathLibrary.ClampAngle` _returnvalue_pitch -20.0 20.0) _returnvalue_yaw) false false)
  (if (not (`self.IsLanding`))
    (`self.K2_SetActorLocation` (`KismetMathLibrary.MakeVector` _returnvalue_x _returnvalue_y (- _returnvalue_z (* DeltaSeconds (`self.FallSpeed`)))))))

(event `self.SupplyBox.OnComponentHit`
  (params (HitComponent :type "PrimitiveComponent Object Reference") (OtherActor :type "Actor Object Reference") (OtherComp :type "PrimitiveComponent Object Reference") (NormalImpulse :type "Vector Structure") (Hit :type "HitResult Structure (by ref)"))
  (`/Engine/EditorBlueprintResources/StandardMacros.DoOnce` false
    (:`Completed`
      (`self.Landing`))))

(event `Landing`
  (set `self.IsLanding` true)
  (`PhysicsConstraintComponent.BreakConstraint` (`self.PhysicsConstraint`))
  (`ActorComponent.K2_DestroyComponent` (`self.Cloth`))
  (for _array_element (`|MakeArray` (`self.Rope1`) (`self.Rope2`) (`self.Rope3`) (`self.Rope4`) (`self.Rope5`) (`self.Rope6`) (`self.Rope7`) (`self.Rope8`) (`self.Rope9`) (`self.Rope10`))
    (`ActorComponent.K2_DestroyComponent` _array_element)
    (`KismetSystemLibrary.Delay` 0.5)
    (`PrimitiveComponent.SetSimulatePhysics` (`self.SupplyBox`) false)))

(event `self.ReceiveActorBeginOverlap`
  (params (OtherActor :type "Actor Object Reference"))
  (bind _asmy_character (cast `MyCharacter` OtherActor))
  (`MyCharacter.SetCanFarmItem` _asmy_character self))

(event `self.ReceiveActorEndOverlap`
  (params (OtherActor :type "Actor Object Reference"))
  (bind _asmy_character (cast `MyCharacter` OtherActor))
  (`MyCharacter.SetCanFarmItem` _asmy_character null))

(fn `UserConstructionScript`)