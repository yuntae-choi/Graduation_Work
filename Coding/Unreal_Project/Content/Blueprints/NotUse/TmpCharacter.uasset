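; Temporary character Blueprint that fakes animation on the head and right upper arm by flipping through 23 component frames each.
; BeginPlay builds both component arrays and starts a looping timer for each, which hides the previous frame and shows the current one.
; The head sequence stops advancing at its last frame, raising material Emissive with the frame index.
; The arm sequence wraps around, snapping each shown frame to a Mesh socket.
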(event `CustomEvent_0`
  (switch `int` (`self.frame`)
    (:`0`
      _)
    (:`1`
      _)
    (:`2`
      _)
    (:`3`
      _)
    (:`4`
      _)
    (:`5`
      _)
    (:`6`
      _)
    (:`7`
      _)
    (:`8`
      _)
    (:`9`
      _)
    (:`10`
      _)
    (:`11`
      _)
    (:`12`
      _)
    (:`13`
      _)
    (:`14`
      _)
    (:`15`
      _)
    (:`16`
      _)
    (:`17`
      _)
    (:`18`
      _)
    (:`19`
      _)
    (:`20`
      _)
    (:`21`
      _)
    (:`22`
      _))
  (if (not (== (`self.frame`) 0))
    (`SceneComponent.SetVisibility` (`|GetArrayItem` (`self.Array`) (- (`self.frame`) 1)) false false))
  (`SceneComponent.SetVisibility` (`|GetArrayItem` (`self.Array`) (`self.frame`)) true false)
  (bind _returnvalue (`PrimitiveComponent.CreateDynamicMaterialInstance` (`|GetArrayItem` (`self.Array`) (`self.frame`)) 1 null "None"))
  (`MaterialInstanceDynamic.SetScalarParameterValue` _returnvalue "Emissive" (* (`self.frame`) 0.125))
  (if (not (== (`self.frame`) (- (`KismetArrayLibrary.Array_Length` (`self.Array`)) 1)))
    (set `self.frame` (+ (`self.frame`) 1))))

(event `self.ReceiveBeginPlay`
  (`|ExecutionSequence`
    (:`then_0`
      (set `self.Array` (`|MakeArray` (`self.head1`) (`self.head2`) (`self.head3`) (`self.head4`) (`self.head5`) (`self.head6`) (`self.head7`) (`self.head8`) (`self.head9`) (`self.head10`) (`self.head11`) (`self.head12`) (`self.head13`) (`self.head14`) (`self.head15`) (`self.head16`) (`self.head17`) (`self.head18`) (`self.head19`) (`self.head20`) (`self.head21`) (`self.head22`) (`self.head23`)))
      (`KismetSystemLibrary.K2_SetTimerDelegate` (delegate `CustomEvent_0`) 0.1 true))
    (:`then_1`
      (set `self.Array2` (`|MakeArray` (`self.rightUpperArm1`) (`self.rightUpperArm2`) (`self.rightUpperArm3`) (`self.rightUpperArm4`) (`self.rightUpperArm5`) (`self.rightUpperArm6`) (`self.rightUpperArm7`) (`self.rightUpperArm8`) (`self.rightUpperArm9`) (`self.rightUpperArm10`) (`self.rightUpperArm11`) (`self.rightUpperArm12`) (`self.rightUpperArm13`) (`self.rightUpperArm14`) (`self.rightUpperArm15`) (`self.rightUpperArm16`) (`self.rightUpperArm17`) (`self.rightUpperArm18`) (`self.rightUpperArm19`) (`self.rightUpperArm20`) (`self.rightUpperArm21`) (`self.rightUpperArm22`) (`self.rightUpperArm23`)))
      (`KismetSystemLibrary.K2_SetTimerDelegate` (delegate `CustomEvent_1`) 0.1 true))))

(event `CustomEvent_1`
  (bind _array2 (`self.Array2`))
  (bind _output (`|GetArrayItem` (`self.Array2`) (`self.frame2`)))
  (switch `int` (`self.frame2`)
    (:`0`
      _)
    (:`1`
      _)
    (:`2`
      _)
    (:`3`
      _)
    (:`4`
      _)
    (:`5`
      _)
    (:`6`
      _)
    (:`7`
      _)
    (:`8`
      _)
    (:`9`
      _)
    (:`10`
      _)
    (:`11`
      _)
    (:`12`
      _)
    (:`13`
      _)
    (:`14`
      _)
    (:`15`
      _)
    (:`16`
      _)
    (:`17`
      _)
    (:`18`
      _)
    (:`19`
      _)
    (:`20`
      _)
    (:`21`
      _)
    (:`22`
      _))
  (if (== (`self.frame2`) 0)
    (`SceneComponent.SetVisibility` (`|GetArrayItem` _array2 (- (`KismetArrayLibrary.Array_Length` _array2) 1)) false false)
    (else
      (`SceneComponent.SetVisibility` (`|GetArrayItem` (`self.Array2`) (- (`self.frame2`) 1)) false false)))
  (`SceneComponent.SetVisibility` _output true false)
  (`SceneComponent.K2_AttachToComponent` _output (`self.Mesh`) "RightUpperarmSocket" "SnapToTarget" "KeepRelative" "KeepRelative" false)
  (if (== (`self.frame2`) (- (`KismetArrayLibrary.Array_Length` (`self.Array2`)) 1))
    (set `self.frame2` 0)
    (else
      (set `self.frame2` (+ (`self.frame2`) 1)))))

(fn `UserConstructionScript`)