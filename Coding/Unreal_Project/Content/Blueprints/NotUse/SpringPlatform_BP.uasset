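; Spring launch platform that flings a ThirdPersonCharacter upward when it enters the Box trigger.
; The overlap adds a velocity-change impulse with a strong vertical kick and amplified horizontal velocity, and prints that velocity for debugging.
; It also starts a Tick-driven state machine that stretches the spring mesh and raises the platform mesh in fixed per-frame steps, holds briefly, then retracts both.
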(event `self.ReceiveBeginPlay`)

(event `self.ReceiveActorBeginOverlap`
  (params (OtherActor :type "Actor Object Reference")))

(event `self.ReceiveTick`
  (params (DeltaSeconds :type "Float (single-precision)"))
  (switch `int` (`self.state`)
    (:`1`
      (if (< (`self.scaleZ`) 3.0)
        (bind _output_get (set `self.scaleZ` (+ (`self.scaleZ`) 0.25)))
        (`SceneComponent.SetWorldScale3D` (`self.SpringMesh`) (`KismetMathLibrary.MakeVector` 1.0 1.0 _output_get))
        (bind _output_get_2 (set `self.platformLocationZ` (+ (`self.platformLocationZ`) 12.25)))
        (`SceneComponent.K2_SetRelativeLocation` (`self.PlatformMesh`) (`KismetMathLibrary.MakeVector` 0.0 0.0 (+ _output_get_2 74.0)) false false)
        (else
          (set `self.state` 3)
          (`KismetSystemLibrary.Delay` 2.0)
          (set `self.state` 2))))
    (:`2`
      (if (> (`self.scaleZ`) 1.0)
        (bind _output_get_3 (set `self.scaleZ` (- (`self.scaleZ`) 0.25)))
        (`SceneComponent.SetWorldScale3D` (`self.SpringMesh`) (`KismetMathLibrary.MakeVector` 1.0 1.0 _output_get_3))
        (bind _output_get_4 (set `self.platformLocationZ` (- (`self.platformLocationZ`) 12.25)))
        (`SceneComponent.K2_SetRelativeLocation` (`self.PlatformMesh`) (`KismetMathLibrary.MakeVector` 0.0 0.0 (+ _output_get_4 74.0)) false false)
        (else
          (set `self.state` 0))))))

(event `self.Box.OnComponentBeginOverlap`
  (params (OverlappedComponent :type "PrimitiveComponent Object Reference") (OtherActor :type "Actor Object Reference") (OtherComp :type "PrimitiveComponent Object Reference") (OtherBodyIndex :type Integer) (bFromSweep :type Boolean) (SweepResult :type "HitResult Structure (by ref)"))
  (bind _asthird_person_character (cast `/Game/ThirdPersonBP/Blueprints/ThirdPersonCharacter` OtherActor))
  (set `self.state` 1)
  (bind (_returnvalue_x _returnvalue_y) (`KismetMathLibrary.BreakVector` (`self.GetVelocity` _asthird_person_character)))
  (`CharacterMovementComponent.AddImpulse` (`Character.CharacterMovement` _asthird_person_character) (`KismetMathLibrary.MakeVector` (* _returnvalue_x 3.0) (* _returnvalue_y 3.0) 3000.0) true)
  (`KismetSystemLibrary.PrintString` (`KismetTextLibrary.Conv_TextToString` (`|FormatText` "{1}, {2}" _returnvalue_x _returnvalue_y))))

(fn `UserConstructionScript`)