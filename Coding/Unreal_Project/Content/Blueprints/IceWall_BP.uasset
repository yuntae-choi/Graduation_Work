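; IceWall_BP is a temporary ice wall actor that rises, stands for a set time, then shatters.
; BeginPlay flattens the DestructibleComponent's Z scale to zero, and Tick raises it by GrowingAmount each frame until full height.
; A DoOnce then waits SpawnDuration and damages the destructible with an impulse along the Arrow component's forward vector.
; The actor destroys itself a few seconds after that hit.
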(event `self.ReceiveBeginPlay`
  (`SceneComponent.SetWorldScale3D` (`self.DestructibleComponent`) (1.0 1.0 0.0)))

(event `self.ReceiveTick`
  (params (DeltaSeconds :type "Float (single-precision)"))
  (bind _arrow (`self.Arrow`))
  (bind (_returnvalue_x _returnvalue_y _returnvalue_z) (`KismetMathLibrary.BreakVector` (`SceneComponent.K2_GetComponentScale` (`self.DestructibleComponent`))))
  (if (< _returnvalue_z 1.0)
    (`SceneComponent.SetWorldScale3D` (`self.DestructibleComponent`) (`KismetMathLibrary.MakeVector` 1.0 1.0 (+ _returnvalue_z (`self.GrowingAmount`))))
    (else
      (`/Engine/EditorBlueprintResources/StandardMacros.DoOnce` false
        (:`Completed`
          (`KismetSystemLibrary.Delay` (`self.SpawnDuration`))
          (`DestructibleComponent.ApplyDamage` (`self.DestructibleComponent`) 1500.0 (`SceneComponent.K2_GetComponentLocation` _arrow) (`SceneComponent.GetForwardVector` _arrow) 1500.0)
          (`KismetSystemLibrary.Delay` 4.0)
          (`self.K2_DestroyActor`))))))

(fn `UserConstructionScript`)