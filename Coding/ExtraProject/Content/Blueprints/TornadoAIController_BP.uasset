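; AI controller for TornadoAI_BP pawns that moves a tornado around a looping patrol path.
; On BeginPlay it reads the spline from the tornado's assigned Path and caches its point count.
; A recursive MoveToNextPoint event sends the pawn to each spline point with AI MoveTo, wrapping to the first after the last.
; The next move starts only on success; failed moves are not retried.
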(event `self.ReceiveBeginPlay`
  (bind _astornado_ai_bp (cast `/Game/Blueprints/TornadoAI_BP` (`self.K2_GetPawn`)))
  (bind _output_get (set `self.Tornado` _astornado_ai_bp))
  (bind _path (`/Game/Blueprints/TornadoAI_BP.Path` _output_get))
  (`/Engine/EditorBlueprintResources/StandardMacros.IsValid` _path
    (:`Is Valid`
      (bind _output_get_2 (set `self.Spline` (`/Game/Blueprints/TornadoPath.Spline` _path)))
      (set `self.NumPoints` (`SplineComponent.GetNumberOfSplinePoints` _output_get_2))
      (`self.MoveToNextPoint`))))

(event `MoveToNextPoint`
  (bind _output_get (set `self.PointIndex` (mod (+ (`self.PointIndex`) 1) (`self.NumPoints`))))
  (`|AIMoveTo` (`self.K2_GetPawn`) (`SplineComponent.GetLocationAtSplinePoint` (`self.Spline`) _output_get "World") null 110.0
    (:`OnSuccess`
      (`self.MoveToNextPoint`))))

(fn `UserConstructionScript`)